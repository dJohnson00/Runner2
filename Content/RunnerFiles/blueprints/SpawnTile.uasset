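; Endless runner floor tile that extends the track when the player reaches its trigger box and fills three lanes with pickups and obstacles.
; On character overlap it has the game mode spawn the next tile, adds multiplied points, nudges walk speed up within a clamp, then destroys itself after a delay.
; SpawnObstables re-rolls randomly per check to place coins, boxes or middle-lane cylinders; an empty lane ends the left-to-right chain.
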(event OnComponentBeginOverlap(Box)
  (params (OverlappedComponent :type Primitive%20Component%20Object%20Reference) (OtherActor :type Actor%20Object%20Reference) (OtherComp :type Primitive%20Component%20Object%20Reference) (OtherBodyIndex :type Integer) (bFromSweep :type Boolean) (SweepResult :type Hit%20Result%20Structure%20%28by%20ref%29))
  (Utilities|Casting|CastToThirdPersonCharacter OtherActor)
  (bind _asthird_person_game_mode (Utilities|Casting|CastToThirdPersonGameMode (Game|GetGameMode)))
  (Default|SpawnTile _asthird_person_game_mode)
  (bind _asthird_person_game_mode_2 (Utilities|Casting|CastToThirdPersonGameMode (Game|GetGameMode)))
  (bind _output_get (Variables|/Game/ThirdPersonBP/Blueprints/ThirdPersonGameMode.ThirdPersonGameMode_C|SetCurrentPoints _asthird_person_game_mode_2 (+ (* 1 (Variables|/Game/ThirdPersonBP/Blueprints/ThirdPersonGameMode.ThirdPersonGameMode_C|GetPointsMultipier _asthird_person_game_mode_2)) (Variables|/Game/ThirdPersonBP/Blueprints/ThirdPersonGameMode.ThirdPersonGameMode_C|GetCurrentPoints _asthird_person_game_mode_2))))
  (Development|PrintString (Utilities|String|ToString(Integer) _output_get))
  (bind _asthird_person_character (Utilities|Casting|CastToThirdPersonCharacter (Game|GetPlayerCharacter 0)))
  (Variables|/Script/Engine.CharacterMovementComponent|SetMaxWalkSpeed (Variables|/Script/Engine.Character|GetCharacterMovement _asthird_person_character) (Math|Float|Clamp(Float) (* (Variables|/Script/Engine.CharacterMovementComponent|GetMaxWalkSpeed (Variables|/Script/Engine.Character|GetCharacterMovement _asthird_person_character)) 1.01) 6e+02 1.2e+03))
  (Utilities|FlowControl|Delay 0.5)
  (Actor|DestroyActor))

(event EventBeginPlay)

(event Collision|EventActorBeginOverlap
  (params (OtherActor :type Actor%20Object%20Reference)))

(event EventTick
  (params (DeltaSeconds :type Float%20%28single-precision%29)))

(fn ConstructionScript)

(fn SpawnObstables
  (bind _returnvalue (Math|Random|RandomFloat))
  (bind _returnvalue_2 (Math|Random|RandomFloat))
  (bind _returnvalue_3 (Math|Random|RandomFloat))
  (bind _laneleft (Variables|Default|GetLaneLeft))
  (bind _lanemiddle (Variables|Default|GetLaneMiddle))
  (bind _laneright (Variables|Default|GetLaneRight))
  (bind _returnvalue_4 (Transformation|GetWorldTransform _laneleft))
  (bind _returnvalue_5 (Transformation|GetWorldTransform _laneright))
  (bind _returnvalue_6 (Transformation|GetWorldTransform _lanemiddle))
  ;[1 1 1] Left Lane
  (if (Math|Float|InRange(Float) _returnvalue 0.0 0.5)
    (Game|SpawnActorfromClass "/Game/RunnerFiles/blueprints/Coin.Coin_C" _returnvalue_4 "Undefined" 0 0)
    ;[1 1 1] Middle Lane
    (if (Math|Float|InRange(Float) _returnvalue_2 0.0 0.4) :!label _label
      (Game|SpawnActorfromClass "/Game/RunnerFiles/blueprints/cylender.cylender_C" _returnvalue_6 "Undefined" 0 0)
      ;[1 1 1] Right Lane
      (if (Math|Float|InRange(Float) _returnvalue_3 0.0 0.5) :!label _label_2
        (Game|SpawnActorfromClass "/Game/RunnerFiles/blueprints/Coin.Coin_C" _returnvalue_5 "Undefined" 0 0)
        (elif (Math|Float|InRange(Float) _returnvalue_3 0.5 0.7)
          (Game|SpawnActorfromClass "/Game/RunnerFiles/blueprints/Obstacle_Box.Obstacle_Box_C" _returnvalue_5 "Undefined" 0 0)
          (elif (Math|Float|InRange(Float) _returnvalue_3 0.8 1.0)
            (Game|SpawnActorfromClass "/Game/RunnerFiles/blueprints/Coin.Coin_C" _returnvalue_5 "Undefined" 0 0))))
      (elif (Math|Float|InRange(Float) _returnvalue_2 0.5 0.7)
        (Game|SpawnActorfromClass "/Game/RunnerFiles/blueprints/Obstacle_Box.Obstacle_Box_C" _returnvalue_6 "Undefined" 0 0)
        (goto _label_2)
        (elif (Math|Float|InRange(Float) _returnvalue_2 0.8 1.0)
          (Game|SpawnActorfromClass "/Game/RunnerFiles/blueprints/Coin.Coin_C" _returnvalue_6 "Undefined" 0 0)
          (goto _label_2))))
    (elif (Math|Float|InRange(Float) _returnvalue 0.5 0.7)
      (Game|SpawnActorfromClass "/Game/RunnerFiles/blueprints/Obstacle_Box.Obstacle_Box_C" _returnvalue_4 "Undefined" 0 0)
      (goto _label)
      (elif (Math|Float|InRange(Float) _returnvalue 0.8 1.0)
        (Game|SpawnActorfromClass "/Game/RunnerFiles/blueprints/Coin.Coin_C" _returnvalue_4 "Undefined" 0 0)
        (goto _label)))))