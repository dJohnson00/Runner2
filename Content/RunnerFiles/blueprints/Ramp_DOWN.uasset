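; Downward ramp piece for a runner game that randomly populates its three bottom lanes with Pole obstacles.
; On BeginPlay it runs SpawnObstacleDownward before calling the parent BeginPlay.
; Each lane rolls a random float for a roughly even chance of a Pole at that lane's component transform.
; A shared NumberOfPillars counter blocks spawns once above one, limiting poles so a lane stays open.
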(event EventBeginPlay
  (CallFunction|SpawnObstacleDownward)
  (|CallParentFunction))

(event Collision|EventActorBeginOverlap
  (params (OtherActor :type Actor%20Object%20Reference))
  (|CallParentFunction OtherActor) ; This node is disabled and will not be called.\nDrag off pins to build functionality.
)

(event EventTick
  (params (DeltaSeconds :type Float%20%28single-precision%29))
  (|CallParentFunction DeltaSeconds) ; This node is disabled and will not be called.\nDrag off pins to build functionality.
)

(fn ConstructionScript
  (|CallParentFunction))

(fn SpawnObstacleDownward
  ;[1 1 1] Left Lane
  (if (Math|Float|InRange(Float) (Math|Random|RandomFloat) 0.0 0.5)
    (if (> (Variables|Default|GetnumberOfPillars) 1)
      (Variables|Default|SetnumberOfPillars 0)
      (else
        (Variables|Default|SetnumberOfPillars (+ (Variables|Default|GetnumberOfPillars) 1))
        (Game|SpawnActorfromClass "/Game/RunnerFiles/blueprints/Pole.Pole_C" (Transformation|GetWorldTransform (Variables|Default|GetLaneBottomLeft)) "Undefined" 0 0))))
  ;[1 1 1] Middle Lane
  (if (Math|Float|InRange(Float) (Math|Random|RandomFloat) 0.0 0.5)
    (if (> (Variables|Default|GetnumberOfPillars) 1)
      (Variables|Default|SetnumberOfPillars 0)
      (else
        (Variables|Default|SetnumberOfPillars (+ (Variables|Default|GetnumberOfPillars) 1))
        (Game|SpawnActorfromClass "/Game/RunnerFiles/blueprints/Pole.Pole_C" (Transformation|GetWorldTransform (Variables|Default|GetLaneBottomMiddle)) "Undefined" 0 0))))
  ;[1 1 1] Right Lane
  (if (Math|Float|InRange(Float) (Math|Random|RandomFloat) 0.0 0.5)
    (if (not (> (Variables|Default|GetnumberOfPillars) 1))
      (Variables|Default|SetnumberOfPillars (+ (Variables|Default|GetnumberOfPillars) 1))
      (Game|SpawnActorfromClass "/Game/RunnerFiles/blueprints/Pole.Pole_C" (Transformation|GetWorldTransform (Variables|Default|GetLaneBottomRight)) "Undefined" 0 0))))